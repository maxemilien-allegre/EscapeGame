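; Key pickup actor that records one of four keys on the first-person player character when interacted with, then destroys itself.
; Its IsKey flags select which character boolean to set, defaulting to Key4.
; Holding keys 1 and 2 lets the referenced BPDoor open, otherwise that pair prints a French missing-key message.
; Holding keys 3 and 4 only prints an all-keys message.
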(event EventBeginPlay)

(event Collision|EventActorBeginOverlap
  (params (OtherActor :type Actor%20Object%20Reference)))

(event EventTick
  (params (DeltaSeconds :type Float%20%28single-precision%29)))

(event EventInteraction
  (Utilities|FlowControl|Sequence
    (:then_0
      (bind _asbp_first_person_character (Utilities|Casting|CastToBP_FirstPersonCharacter (Game|GetPlayerCharacter 0)))
      (if (Variables|Default|GetIsKey1)
        (Variables|/Game/Blueprints/Implemented/BP_FirstPersonCharacter.BP_FirstPersonCharacter_C|SetKey1 _asbp_first_person_character true)
        (if (and (Variables|/Game/Blueprints/Implemented/BP_FirstPersonCharacter.BP_FirstPersonCharacter_C|GetKey1 _asbp_first_person_character) (Variables|/Game/Blueprints/Implemented/BP_FirstPersonCharacter.BP_FirstPersonCharacter_C|GetKey2 _asbp_first_person_character)) :!label _label
          (Variables|/Game/Door_aperture_2_Blueprint.Door_aperture_2_Blueprint_C|SetCanOpen (Variables|Default|GetBP_Door) true)
          (else
            (Development|PrintString "Il me manque une clé")))
        (elif (Variables|Default|GetIsKey2)
          (Variables|/Game/Blueprints/Implemented/BP_FirstPersonCharacter.BP_FirstPersonCharacter_C|SetKey2 _asbp_first_person_character true)
          (goto _label)
          (else
            (if (Variables|Default|GetIsKey3)
              (Variables|/Game/Blueprints/Implemented/BP_FirstPersonCharacter.BP_FirstPersonCharacter_C|SetKey3 _asbp_first_person_character true)
              (else
                (Variables|/Game/Blueprints/Implemented/BP_FirstPersonCharacter.BP_FirstPersonCharacter_C|SetKey4 _asbp_first_person_character true)))
            (if (and (Variables|/Game/Blueprints/Implemented/BP_FirstPersonCharacter.BP_FirstPersonCharacter_C|GetKey3 _asbp_first_person_character) (Variables|/Game/Blueprints/Implemented/BP_FirstPersonCharacter.BP_FirstPersonCharacter_C|GetKey4 _asbp_first_person_character))
              (Development|PrintString "J'ai toutes les clés !"))))))
    (:then_1
      (Actor|DestroyActor))))

(fn ConstructionScript)